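; BP_BlinkLight is an actor whose point light flickers at random intervals.
; From BeginPlay, the BlinkLight event switches the light off for a brief random delay, then back to full intensity for a longer random delay of up to several seconds.
; The event then calls itself, forming an endless loop without Tick or a timeline.
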(event Custom|BlinkLight
  (Rendering|Components|Light|SetIntensity (Variables|Default|GetPointLight) 0.0)
  (Utilities|FlowControl|Delay (Math|Random|RandomFloatinRange 0.1 0.3))
  (Rendering|Components|Light|SetIntensity (Variables|Default|GetPointLight) 5e+02)
  (Utilities|FlowControl|Delay (Math|Random|RandomFloatinRange 0.0 7.0))
  (CallFunction|BlinkLight))

(event EventBeginPlay
  (CallFunction|BlinkLight))

(fn ConstructionScript)